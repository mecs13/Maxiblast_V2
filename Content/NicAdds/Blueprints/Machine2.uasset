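; Machine actor, apparently a screw (Vite) cleaning station for the VR game, with functions to show the Vite component and change its material.
; The VR pawn entering Box plays the screw cleaning system sound, guarded by a DoOnce.
; Door-opening timeline, spray toggling and game-instance check for the taken screw are disconnected, leaving their overlap and Tick events empty.
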(event `self.ReceiveBeginPlay`)

(event `self.overlapOpenDoor.OnComponentBeginOverlap`
  (params (OverlappedComponent :type "PrimitiveComponent Object Reference") (OtherActor :type "Actor Object Reference") (OtherComp :type "PrimitiveComponent Object Reference") (OtherBodyIndex :type Integer) (bFromSweep :type Boolean) (SweepResult :type "HitResult Structure (by ref)")))

(event `self.ReceiveTick`
  (params (DeltaSeconds :type "Float (single-precision)"))
  ;[1 1 1] Show big piece in the machine
)

(event `self.overlapForSpray.OnComponentBeginOverlap`
  (params (OverlappedComponent :type "PrimitiveComponent Object Reference") (OtherActor :type "Actor Object Reference") (OtherComp :type "PrimitiveComponent Object Reference") (OtherBodyIndex :type Integer) (bFromSweep :type Boolean) (SweepResult :type "HitResult Structure (by ref)")))

(event `self.overlapForSpray.OnComponentEndOverlap`
  (params (OverlappedComponent :type "PrimitiveComponent Object Reference") (OtherActor :type "Actor Object Reference") (OtherComp :type "PrimitiveComponent Object Reference") (OtherBodyIndex :type Integer)))

(event `self.Box.OnComponentBeginOverlap`
  (params (OverlappedComponent :type "PrimitiveComponent Object Reference") (OtherActor :type "Actor Object Reference") (OtherComp :type "PrimitiveComponent Object Reference") (OtherBodyIndex :type Integer) (bFromSweep :type Boolean) (SweepResult :type "HitResult Structure (by ref)"))
  (bind _asvrpawn (cast `/Game/VRTemplate/Blueprints/VRPawn` (`GameplayStatics.GetPlayerPawn` 0)))
  (if (== OtherActor _asvrpawn)
    (`/Engine/EditorBlueprintResources/StandardMacros.DoOnce` false
      (:`Completed`
        (`GameplayStatics.PlaySound2D` "/Game/NicAdds/sounds/mobilescrewcleaningsystem.mobilescrewcleaningsystem" 1.0 1.0 0.0 null null)))))

(fn `changeViteMaterial`
  (params (viteMaterial :type "MaterialInstance Object Reference"))
  (`PrimitiveComponent.SetMaterial` (`self.vite`) 0 viteMaterial))

(fn `showVite`
  (`SceneComponent.SetHiddenInGame` (`self.vite`) false false))

(fn `UserConstructionScript`)