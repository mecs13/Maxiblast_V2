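; Trigger actor for the third mesh option, selected when the player's VR pawn overlaps its Box component.
; Each player overlap sets WokingMesh to 3 on the P_GameInstance.
; A DoOnce with no reset limits the feedback to the first overlap: a click sound and a call to ChangeViteMaterial on Machine1 with a scratched painted iron material.
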(event `self.Box.OnComponentBeginOverlap`
  (params (OverlappedComponent :type "PrimitiveComponent Object Reference") (OtherActor :type "Actor Object Reference") (OtherComp :type "PrimitiveComponent Object Reference") (OtherBodyIndex :type Integer) (bFromSweep :type Boolean) (SweepResult :type "HitResult Structure (by ref)"))
  (bind _asvrpawn (cast `/Game/VRTemplate/Blueprints/VRPawn` (`GameplayStatics.GetPlayerPawn` 0)))
  (if (== _asvrpawn OtherActor)
    (bind _asp_game_instance (cast `/Game/NicAdds/P_GameInstance` (`GameplayStatics.GetGameInstance`)))
    (set `/Game/NicAdds/P_GameInstance.wokingMesh` 3 _asp_game_instance)
    (`/Engine/EditorBlueprintResources/StandardMacros.DoOnce` false
      (:`Completed`
        (`GameplayStatics.PlaySound2D` "/Game/SoundsEffect/widgetClick.widgetClick" 1.0 1.0 0.0 null null)
        (bind _returnvalue (`GameplayStatics.GetActorOfClass` "/Game/NicAdds/Blueprints/Machine1.Machine1_C"))
        (`/Game/NicAdds/Blueprints/Machine1.changeViteMaterial` _returnvalue "/Game/Megascans/Surfaces/Scratched_Painted_Iron_scksebop/MI_Scratched_Painted_Iron_scksebop_1K.MI_Scratched_Painted_Iron_scksebop_1K")))))

(fn `UserConstructionScript`)