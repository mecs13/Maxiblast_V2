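; Machine actor for a VR scene, apparently a pressure-blast stripping station, that displays the current workpiece and lets the player spray.
; Every Tick it shows one of four models from the game instance's WokingMesh index, while overlap volumes play a one-time sound and toggle the VRPawn's spray.
; Functions swap model materials, stepped by the game instance's NClick, and reveal Plane or Vite.
; Door-opening timeline logic remains but never runs.
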(event `self.machineOverlap.OnComponentBeginOverlap`
  (params (OverlappedComponent :type "PrimitiveComponent Object Reference") (OtherActor :type "Actor Object Reference") (OtherComp :type "PrimitiveComponent Object Reference") (OtherBodyIndex :type Integer) (bFromSweep :type Boolean) (SweepResult :type "HitResult Structure (by ref)"))
  (bind _asvrpawn (cast `/Game/VRTemplate/Blueprints/VRPawn` (`GameplayStatics.GetPlayerPawn` 0)))
  (if (== OtherActor _asvrpawn)
    (`/Engine/EditorBlueprintResources/StandardMacros.DoOnce` false
      (:`Completed`
        (`GameplayStatics.PlaySound2D` "/Game/NicAdds/sounds/pressureblaststrippingsystem.pressureblaststrippingsystem" 1.0 1.0 0.0 null null)))))

(event `self.ReceiveBeginPlay`)

(event `self.ReceiveTick`
  (params (DeltaSeconds :type "Float (single-precision)"))
  (bind _model (`self.model`))
  (bind _model1 (`self.model1`))
  (bind _model2 (`self.model2`))
  (bind _model3 (`self.model3`))
  ;[1 1 1] Show big piece in the machine
  (bind _asp_game_instance (cast `/Game/NicAdds/P_GameInstance` (`GameplayStatics.GetGameInstance`)))
  (switch `int` (`/Game/NicAdds/P_GameInstance.wokingMesh` _asp_game_instance)
    (:`0`
      (set `self.ChosenOne` _model)
      (`SceneComponent.SetHiddenInGame` _model false false)
      (`SceneComponent.SetHiddenInGame` (`self.model2`) true false)
      (`SceneComponent.SetHiddenInGame` (`self.model1`) true false)
      (`SceneComponent.SetHiddenInGame` (`self.model3`) true false))
    (:`1`
      (set `self.ChosenOne` _model1)
      (`SceneComponent.SetHiddenInGame` _model1 false false)
      (`SceneComponent.SetHiddenInGame` (`self.model3`) true false)
      (`SceneComponent.SetHiddenInGame` (`self.model2`) true false)
      (`SceneComponent.SetHiddenInGame` (`self.model`) true false))
    (:`2`
      (set `self.ChosenOne` _model2)
      (`SceneComponent.SetHiddenInGame` _model2 false false)
      (`SceneComponent.SetHiddenInGame` (`self.model3`) true false)
      (`SceneComponent.SetHiddenInGame` (`self.model1`) true false)
      (`SceneComponent.SetHiddenInGame` (`self.model`) true false))
    (:`3`
      (set `self.ChosenOne` _model3)
      (`SceneComponent.SetHiddenInGame` _model3 false false)
      (`SceneComponent.SetHiddenInGame` (`self.model2`) true false)
      (`SceneComponent.SetHiddenInGame` (`self.model1`) true false)
      (`SceneComponent.SetHiddenInGame` (`self.model`) true false))))

(event `self.overlapForSpray.OnComponentBeginOverlap`
  (params (OverlappedComponent :type "PrimitiveComponent Object Reference") (OtherActor :type "Actor Object Reference") (OtherComp :type "PrimitiveComponent Object Reference") (OtherBodyIndex :type Integer) (bFromSweep :type Boolean) (SweepResult :type "HitResult Structure (by ref)"))
  (bind _asvrpawn (cast `/Game/VRTemplate/Blueprints/VRPawn` (`GameplayStatics.GetPlayerPawn` 0)))
  (`SceneComponent.SetHiddenInGame` (`/Game/VRTemplate/Blueprints/VRPawn.spray` _asvrpawn) false false)
  (set `/Game/VRTemplate/Blueprints/VRPawn.canSpray` true _asvrpawn))

(event `self.overlapForSpray.OnComponentEndOverlap`
  (params (OverlappedComponent :type "PrimitiveComponent Object Reference") (OtherActor :type "Actor Object Reference") (OtherComp :type "PrimitiveComponent Object Reference") (OtherBodyIndex :type Integer))
  (bind _asvrpawn (cast `/Game/VRTemplate/Blueprints/VRPawn` (`GameplayStatics.GetPlayerPawn` 0)))
  (`SceneComponent.SetHiddenInGame` (`/Game/VRTemplate/Blueprints/VRPawn.spray` _asvrpawn) true false)
  (set `/Game/VRTemplate/Blueprints/VRPawn.canSpray` false _asvrpawn))

(fn `changeColor`
  (bind _model2 (`self.model2`))
  (bind _model3 (`self.model3`))
  (bind _asp_game_instance (cast `/Game/NicAdds/P_GameInstance` (`GameplayStatics.GetGameInstance`)))
  (switch `int` (`/Game/NicAdds/P_GameInstance.N_click` _asp_game_instance)
    (:`0`
      (`SceneComponent.SetHiddenInGame` (`self.Plane`) true true))
    (:`1`
      (`PrimitiveComponent.SetMaterial` _model3 0 "/Game/Megascans/Surfaces/Scratched_Painted_Iron_scksebop/MI_step1.MI_step1")
      (`PrimitiveComponent.SetMaterial` (`self.model1`) 0 "/Game/Megascans/Surfaces/Scratched_Painted_Iron_scksebop/MI_step1.MI_step1")
      (`PrimitiveComponent.SetMaterial` (`self.model`) 0 "/Game/Megascans/Surfaces/Scratched_Painted_Iron_scksebop/MI_step1.MI_step1")
      (`PrimitiveComponent.SetMaterial` _model2 0 "/Game/Megascans/Surfaces/Scratched_Painted_Iron_scksebop/MI_step1.MI_step1"))
    (:`2`
      (`PrimitiveComponent.SetMaterial` _model3 0 "/Game/Megascans/Surfaces/Scratched_Painted_Iron_scksebop/MI_step2.MI_step2")
      (`PrimitiveComponent.SetMaterial` (`self.model1`) 0 "/Game/Megascans/Surfaces/Scratched_Painted_Iron_scksebop/MI_step2.MI_step2")
      (`PrimitiveComponent.SetMaterial` (`self.model`) 0 "/Game/Megascans/Surfaces/Scratched_Painted_Iron_scksebop/MI_step2.MI_step2")
      (`PrimitiveComponent.SetMaterial` _model2 0 "/Game/Megascans/Surfaces/Scratched_Painted_Iron_scksebop/MI_step2.MI_step2"))
    (:`3`
      (`PrimitiveComponent.SetMaterial` _model2 0 "/Game/Megascans/Surfaces/Scratched_Painted_Iron_scksebop/MI_step3.MI_step3")
      (`PrimitiveComponent.SetMaterial` (`self.model`) 0 "/Game/Megascans/Surfaces/Scratched_Painted_Iron_scksebop/MI_step3.MI_step3")
      (`PrimitiveComponent.SetMaterial` (`self.model1`) 0 "/Game/Megascans/Surfaces/Scratched_Painted_Iron_scksebop/MI_step3.MI_step3")
      (`PrimitiveComponent.SetMaterial` _model3 0 "/Game/Megascans/Surfaces/Scratched_Painted_Iron_scksebop/MI_step3.MI_step3"))
    (:`4`
      (`PrimitiveComponent.SetMaterial` _model2 0 "/Game/Megascans/Surfaces/Scratched_Painted_Iron_scksebop/MI_step4.MI_step4")
      (`PrimitiveComponent.SetMaterial` (`self.model`) 0 "/Game/Megascans/Surfaces/Scratched_Painted_Iron_scksebop/MI_step4.MI_step4")
      (`PrimitiveComponent.SetMaterial` (`self.model1`) 0 "/Game/Megascans/Surfaces/Scratched_Painted_Iron_scksebop/MI_step4.MI_step4")
      (`PrimitiveComponent.SetMaterial` _model3 0 "/Game/Megascans/Surfaces/Scratched_Painted_Iron_scksebop/MI_step4.MI_step4"))
    (:`5`
      (`PrimitiveComponent.SetMaterial` _model2 0 "/Game/Megascans/Surfaces/Scratched_Painted_Iron_scksebop/MI_step5.MI_step5")
      (`PrimitiveComponent.SetMaterial` (`self.model`) 0 "/Game/Megascans/Surfaces/Scratched_Painted_Iron_scksebop/MI_step5.MI_step5")
      (`PrimitiveComponent.SetMaterial` (`self.model1`) 0 "/Game/Megascans/Surfaces/Scratched_Painted_Iron_scksebop/MI_step5.MI_step5")
      (`PrimitiveComponent.SetMaterial` _model3 0 "/Game/Megascans/Surfaces/Scratched_Painted_Iron_scksebop/MI_step5.MI_step5")
      (`SceneComponent.SetHiddenInGame` (`self.Plane`) false true))))

(fn `changeViteMaterial`
  (params (viteMaterial :type "MaterialInstance Object Reference"))
  (`PrimitiveComponent.SetMaterial` (`self.model3`) 0 viteMaterial)
  (`PrimitiveComponent.SetMaterial` (`self.model2`) 0 viteMaterial)
  (`PrimitiveComponent.SetMaterial` (`self.model1`) 0 viteMaterial)
  (`PrimitiveComponent.SetMaterial` (`self.model`) 0 viteMaterial))

(fn `showVite`
  (`SceneComponent.SetHiddenInGame` (`self.vite`) false false))

(fn `UserConstructionScript`)