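; VR machine actor, apparently for pressure-blast cleaning, with a sliding door and a display of the current work piece.
; Door-trigger overlaps flip a flag, alternately playing a timeline that slides the Scene component with a sound and green sphere (player pawn only), or reversing it for any actor.
; Tick shows one of four piece meshes from the game instance's WokingMesh index.
; Spray overlaps and Vite functions are empty, their logic disconnected.
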(event `self.ReceiveBeginPlay`)

(event `self.overlapOpenDoor.OnComponentBeginOverlap`
  (params (OverlappedComponent :type "PrimitiveComponent Object Reference") (OtherActor :type "Actor Object Reference") (OtherComp :type "PrimitiveComponent Object Reference") (OtherBodyIndex :type Integer) (bFromSweep :type Boolean) (SweepResult :type "HitResult Structure (by ref)"))
  (bind (_returnvalue_x _returnvalue_y _returnvalue_z) (`KismetMathLibrary.BreakVector` (`SceneComponent.K2_GetComponentLocation` (`self.Scene`))))
  (if (`self.forBeh`)
    (set `self.forBeh` false)
    (`PrimitiveComponent.SetMaterial` (`self.Sphere`) 0 "/Engine/MapTemplates/Materials/BasicAsset01.BasicAsset01")
    ;[1 1 1] Open door
    (bind (_direction _movingvalue) (`Timeline|Timeline_0` :!via `Reverse` :!label _label)
      (:`Update`
        (`SceneComponent.K2_SetRelativeLocation` (`self.Scene`) (`KismetMathLibrary.VLerp` (-40.0 -124.0 89.0) (280.0 -124.0 89.0) _movingvalue) false false)))
    (else
      (set `self.forBeh` true)
      (bind _asvrpawn (cast `/Game/VRTemplate/Blueprints/VRPawn` (`GameplayStatics.GetPlayerPawn` 0)))
      (if (== OtherActor _asvrpawn)
        (`GameplayStatics.PlaySound2D` "/Game/NicAdds/sounds/3pressureblastmoldcleaningsystems.3pressureblastmoldcleaningsystems" 1.0 1.0 0.0 null null)
        (`PrimitiveComponent.SetMaterial` (`self.Sphere`) 0 "/Engine/EngineDebugMaterials/VertexColorViewMode_GreenOnly.VertexColorViewMode_GreenOnly")
        (set `self.YRot` _returnvalue_y)
        (set `self.ZRot` _returnvalue_z)
        (goto _label :!via `PlayFromStart`)))))

(event `self.ReceiveTick`
  (params (DeltaSeconds :type "Float (single-precision)"))
  ;[1 1 1] Show big piece in the machine
  (bind _asp_game_instance (cast `/Game/NicAdds/P_GameInstance` (`GameplayStatics.GetGameInstance`)))
  (switch `int` (`/Game/NicAdds/P_GameInstance.wokingMesh` _asp_game_instance)
    (:`0`
      (`SceneComponent.SetHiddenInGame` (`self.0`) false false)
      (`SceneComponent.SetHiddenInGame` (`self.2`) true false)
      (`SceneComponent.SetHiddenInGame` (`self.3`) true false)
      (`SceneComponent.SetHiddenInGame` (`self.1`) true false))
    (:`1`
      (`SceneComponent.SetHiddenInGame` (`self.1`) false false)
      (`SceneComponent.SetHiddenInGame` (`self.2`) true false)
      (`SceneComponent.SetHiddenInGame` (`self.3`) true false)
      (`SceneComponent.SetHiddenInGame` (`self.0`) true false))
    (:`2`
      (`SceneComponent.SetHiddenInGame` (`self.2`) false false)
      (`SceneComponent.SetHiddenInGame` (`self.0`) true false)
      (`SceneComponent.SetHiddenInGame` (`self.3`) true false)
      (`SceneComponent.SetHiddenInGame` (`self.1`) true false))
    (:`3`
      (`SceneComponent.SetHiddenInGame` (`self.3`) false false)
      (`SceneComponent.SetHiddenInGame` (`self.1`) true false)
      (`SceneComponent.SetHiddenInGame` (`self.2`) true false)
      (`SceneComponent.SetHiddenInGame` (`self.0`) true false))))

(event `self.overlapForSpray.OnComponentBeginOverlap`
  (params (OverlappedComponent :type "PrimitiveComponent Object Reference") (OtherActor :type "Actor Object Reference") (OtherComp :type "PrimitiveComponent Object Reference") (OtherBodyIndex :type Integer) (bFromSweep :type Boolean) (SweepResult :type "HitResult Structure (by ref)")))

(event `self.overlapForSpray.OnComponentEndOverlap`
  (params (OverlappedComponent :type "PrimitiveComponent Object Reference") (OtherActor :type "Actor Object Reference") (OtherComp :type "PrimitiveComponent Object Reference") (OtherBodyIndex :type Integer)))

(fn `changeViteMaterial`
  (params (viteMaterial :type "MaterialInstance Object Reference")))

(fn `showVite`)

(fn `UserConstructionScript`)