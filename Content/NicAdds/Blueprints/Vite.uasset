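; Vite is a pickup (French for screw) that the VR player collects by touching its box.
; On overlap with the VR pawn it sets a text render's text, destroys itself and flags ViteTaken on the P_GameInstance.
; It then tells the first Machine1 actor in the level to show the Vite.
; The construction script and ChangeMaterial function are empty.
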(event `self.Box.OnComponentBeginOverlap`
  (params (OverlappedComponent :type "PrimitiveComponent Object Reference") (OtherActor :type "Actor Object Reference") (OtherComp :type "PrimitiveComponent Object Reference") (OtherBodyIndex :type Integer) (bFromSweep :type Boolean) (SweepResult :type "HitResult Structure (by ref)"))
  (bind _asvrpawn (cast `/Game/VRTemplate/Blueprints/VRPawn` (`GameplayStatics.GetPlayerPawn` 0)))
  (if (== _asvrpawn OtherActor)
    (`TextRenderComponent.K2_SetText` (`self.TextRender`) (`self.text`))
    (`self.K2_DestroyActor`)
    (bind _asp_game_instance (cast `/Game/NicAdds/P_GameInstance` (`GameplayStatics.GetGameInstance`)))
    (set `/Game/NicAdds/P_GameInstance.viteTaken` true _asp_game_instance)
    (bind _outactors (`GameplayStatics.GetAllActorsOfClass` "/Game/NicAdds/Blueprints/Machine1.Machine1_C"))
    (`/Game/NicAdds/Blueprints/Machine1.showVite` (`|GetArrayItem` _outactors))))

(fn `changeMaterial`)

(fn `UserConstructionScript`)