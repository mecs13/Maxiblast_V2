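; VR button panel for Machine1 that offers Wood, Plastic and Glass choices.
; A right-hand overlap on a button plays a click, simulates a pointer press through the pawn's widget interaction, and highlights one indicator mesh.
; Plastic and Glass store their material and type flags in P_GameInstance; Wood's material assignment is unwired and it sets no flags.
; All three call ChangeViteMaterial on Machine1 with the same painted-iron material.
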(event `self.wood.OnComponentBeginOverlap`
  (params (OverlappedComponent :type "PrimitiveComponent Object Reference") (OtherActor :type "Actor Object Reference") (OtherComp :type "PrimitiveComponent Object Reference") (OtherBodyIndex :type Integer) (bFromSweep :type Boolean) (SweepResult :type "HitResult Structure (by ref)"))
  ;[1 1 1] WoodChosen
  (bind _asvrpawn (cast `/Game/VRTemplate/Blueprints/VRPawn` (`GameplayStatics.GetPlayerPawn` 0)))
  (if (== OtherComp (`/Game/VRTemplate/Blueprints/VRPawn.rightHandColl` _asvrpawn))
    (`GameplayStatics.PlaySound2D` "/Game/SoundsEffect/widgetClick.widgetClick" 1.0 1.0 0.0 null null)
    (bind _widgetinteractionright (`/Game/VRTemplate/Blueprints/VRPawn.WidgetInteractionRight` _asvrpawn))
    (`WidgetInteractionComponent.PressPointerKey` _widgetinteractionright "LeftMouseButton")
    (`KismetSystemLibrary.Delay` 0.2)
    (`WidgetInteractionComponent.ReleasePointerKey` _widgetinteractionright "LeftMouseButton")
    (bind _asp_game_instance (cast `/Game/NicAdds/P_GameInstance` (`GameplayStatics.GetGameInstance`)))
    (`PrimitiveComponent.SetMaterial` (`self.S_black`) 0 "/Engine/VREditor/BasicMeshes/MI_Cube_03.MI_Cube_03")
    (`PrimitiveComponent.SetMaterial` (`self.S_blue`) 0 "/Engine/BasicShapes/BasicShapeMaterial.BasicShapeMaterial")
    (`PrimitiveComponent.SetMaterial` (`self.S_brown`) 0 "/Engine/BasicShapes/BasicShapeMaterial.BasicShapeMaterial")
    (bind _returnvalue (`GameplayStatics.GetActorOfClass` "/Game/NicAdds/Blueprints/Machine1.Machine1_C"))
    (`/Game/NicAdds/Blueprints/Machine1.changeViteMaterial` _returnvalue "/Game/Megascans/Surfaces/Scratched_Painted_Iron_scksebop/MI_Scratched_Painted_Iron_scksebop_1K.MI_Scratched_Painted_Iron_scksebop_1K")))

(event `self.plastic.OnComponentBeginOverlap`
  (params (OverlappedComponent :type "PrimitiveComponent Object Reference") (OtherActor :type "Actor Object Reference") (OtherComp :type "PrimitiveComponent Object Reference") (OtherBodyIndex :type Integer) (bFromSweep :type Boolean) (SweepResult :type "HitResult Structure (by ref)"))
  ;[1 1 1] PlasticChosen
  (bind _asvrpawn (cast `/Game/VRTemplate/Blueprints/VRPawn` (`GameplayStatics.GetPlayerPawn` 0)))
  (if (== OtherComp (`/Game/VRTemplate/Blueprints/VRPawn.rightHandColl` _asvrpawn))
    (`GameplayStatics.PlaySound2D` "/Game/SoundsEffect/widgetClick.widgetClick" 1.0 1.0 0.0 null null)
    (bind _widgetinteractionright (`/Game/VRTemplate/Blueprints/VRPawn.WidgetInteractionRight` _asvrpawn))
    (`WidgetInteractionComponent.PressPointerKey` _widgetinteractionright "LeftMouseButton")
    (`KismetSystemLibrary.Delay` 0.2)
    (`WidgetInteractionComponent.ReleasePointerKey` _widgetinteractionright "LeftMouseButton")
    (bind _asp_game_instance (cast `/Game/NicAdds/P_GameInstance` (`GameplayStatics.GetGameInstance`)))
    (set `/Game/NicAdds/P_GameInstance.viteColor` "/Game/Megascans/Surfaces/Scratched_Painted_Iron_scksebop/MI_Scratched_Painted_Iron_scksebop_1K.MI_Scratched_Painted_Iron_scksebop_1K" _asp_game_instance)
    (`PrimitiveComponent.SetMaterial` (`self.S_blue`) 0 "/Engine/VREditor/BasicMeshes/MI_Cube_03.MI_Cube_03")
    (`PrimitiveComponent.SetMaterial` (`self.S_black`) 0 "/Engine/BasicShapes/BasicShapeMaterial.BasicShapeMaterial")
    (`PrimitiveComponent.SetMaterial` (`self.S_brown`) 0 "/Engine/BasicShapes/BasicShapeMaterial.BasicShapeMaterial")
    (set `/Game/NicAdds/P_GameInstance.isPlastic` true _asp_game_instance)
    (set `/Game/NicAdds/P_GameInstance.isGlass` false _asp_game_instance)
    (bind _returnvalue (`GameplayStatics.GetActorOfClass` "/Game/NicAdds/Blueprints/Machine1.Machine1_C"))
    (`/Game/NicAdds/Blueprints/Machine1.changeViteMaterial` _returnvalue "/Game/Megascans/Surfaces/Scratched_Painted_Iron_scksebop/MI_Scratched_Painted_Iron_scksebop_1K.MI_Scratched_Painted_Iron_scksebop_1K")))

(event `self.glass.OnComponentBeginOverlap`
  (params (OverlappedComponent :type "PrimitiveComponent Object Reference") (OtherActor :type "Actor Object Reference") (OtherComp :type "PrimitiveComponent Object Reference") (OtherBodyIndex :type Integer) (bFromSweep :type Boolean) (SweepResult :type "HitResult Structure (by ref)"))
  ;[1 1 1] GlassChosen
  (bind _asvrpawn (cast `/Game/VRTemplate/Blueprints/VRPawn` (`GameplayStatics.GetPlayerPawn` 0)))
  (if (== OtherComp (`/Game/VRTemplate/Blueprints/VRPawn.rightHandColl` _asvrpawn))
    (`GameplayStatics.PlaySound2D` "/Game/SoundsEffect/widgetClick.widgetClick" 1.0 1.0 0.0 null null)
    (bind _widgetinteractionright (`/Game/VRTemplate/Blueprints/VRPawn.WidgetInteractionRight` _asvrpawn))
    (`WidgetInteractionComponent.PressPointerKey` _widgetinteractionright "LeftMouseButton")
    (`KismetSystemLibrary.Delay` 0.2)
    (`WidgetInteractionComponent.ReleasePointerKey` _widgetinteractionright "LeftMouseButton")
    (bind _asp_game_instance (cast `/Game/NicAdds/P_GameInstance` (`GameplayStatics.GetGameInstance`)))
    (set `/Game/NicAdds/P_GameInstance.viteColor` "/Game/3dModels/Acciaio/M_badMaterial_Inst.M_badMaterial_Inst" _asp_game_instance)
    (`PrimitiveComponent.SetMaterial` (`self.S_brown`) 0 "/Engine/VREditor/BasicMeshes/MI_Cube_03.MI_Cube_03")
    (`PrimitiveComponent.SetMaterial` (`self.S_black`) 0 "/Engine/BasicShapes/BasicShapeMaterial.BasicShapeMaterial")
    (`PrimitiveComponent.SetMaterial` (`self.S_blue`) 0 "/Engine/BasicShapes/BasicShapeMaterial.BasicShapeMaterial")
    (set `/Game/NicAdds/P_GameInstance.isGlass` true _asp_game_instance)
    (set `/Game/NicAdds/P_GameInstance.isPlastic` false _asp_game_instance)
    (bind _returnvalue (`GameplayStatics.GetActorOfClass` "/Game/NicAdds/Blueprints/Machine1.Machine1_C"))
    (`/Game/NicAdds/Blueprints/Machine1.changeViteMaterial` _returnvalue "/Game/Megascans/Surfaces/Scratched_Painted_Iron_scksebop/MI_Scratched_Painted_Iron_scksebop_1K.MI_Scratched_Painted_Iron_scksebop_1K")))

(fn `UserConstructionScript`)