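; BP_chosingPanel is an actor that shows the currently selected big piece in the machine.
; Every tick it reads the WokingMesh index from P_GameInstance and switches on it across four cases.
; Each case unhides the matching component among Model, Model1, Model2 and Model3 and hides the other three, so the display follows the shared state by polling.
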(event `self.ReceiveTick`
  (params (DeltaSeconds :type "Float (single-precision)"))
  ;[1 1 1] Show big piece in the machine
  (bind _asp_game_instance (cast `/Game/NicAdds/P_GameInstance` (`GameplayStatics.GetGameInstance`)))
  (switch `int` (`/Game/NicAdds/P_GameInstance.wokingMesh` _asp_game_instance)
    (:`0`
      (`SceneComponent.SetHiddenInGame` (`self.model`) false false)
      (`SceneComponent.SetHiddenInGame` (`self.model2`) true false)
      (`SceneComponent.SetHiddenInGame` (`self.model1`) true false)
      (`SceneComponent.SetHiddenInGame` (`self.model3`) true false))
    (:`1`
      (`SceneComponent.SetHiddenInGame` (`self.model1`) false false)
      (`SceneComponent.SetHiddenInGame` (`self.model3`) true false)
      (`SceneComponent.SetHiddenInGame` (`self.model2`) true false)
      (`SceneComponent.SetHiddenInGame` (`self.model`) true false))
    (:`2`
      (`SceneComponent.SetHiddenInGame` (`self.model2`) false false)
      (`SceneComponent.SetHiddenInGame` (`self.model3`) true false)
      (`SceneComponent.SetHiddenInGame` (`self.model1`) true false)
      (`SceneComponent.SetHiddenInGame` (`self.model`) true false))
    (:`3`
      (`SceneComponent.SetHiddenInGame` (`self.model3`) false false)
      (`SceneComponent.SetHiddenInGame` (`self.model2`) true false)
      (`SceneComponent.SetHiddenInGame` (`self.model1`) true false)
      (`SceneComponent.SetHiddenInGame` (`self.model`) true false))))

(fn `UserConstructionScript`)